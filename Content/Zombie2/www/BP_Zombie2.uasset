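; BP_Zombie2 is a zombie that chases the first player by moving straight toward them every frame.
; On Tick, a sequence rotates the capsule to the look-at rotation toward the player, then offsets the actor along the capsule's forward vector.
; Movement is a fixed step per frame, with no delta-time scaling, collision sweep or pathfinding.
; BeginPlay, ActorBeginOverlap and the construction script are empty.
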(event EventBeginPlay)

(event Collision|EventActorBeginOverlap
  (params (OtherActor :type Actor%20Object%20Reference)))

(event EventTick
  (params (DeltaSeconds :type Float%20%28single-precision%29))
  (Utilities|FlowControl|Sequence ; 0 먼저 하고  음 1...다음 2.. 실행
    (:then_0
      (Transformation|SetWorldRotation (Variables|Collision|GetCapsuleComponent) (Math|Rotator|FindLookatRotation (Transformation|GetActorLocation) (Transformation|GetActorLocation (Game|GetPlayerCharacter 0))) false false))
    (:then_1
      (Transformation|SetActorLocation (+ (Transformation|GetActorLocation) (* (Math|Vector|GetForwardVector (Variables|Collision|GetCapsuleComponent)) 2.0)) false false) ; 캐릭 위치 + 방향 값으로 위치 변화
    )))

(fn ConstructionScript)